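; BP_CAttachment_MagicBall is an attachment that shows a magic ball particle effect at the character's Hand_ThrowItem socket.
; On BeginPlay it attaches its ParticleSystem to that socket.
; Equipping activates the particles and plays a timeline that drives their relative scale, while unequipping deactivates them.
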(event EventBeginPlay
  (Class|CAttachment|ComponentAttachto (Variables|Default|GetParticleSystem) "Hand_ThrowItem"))

(event EventOnEquip
  (Components|Activation|SetActive (Variables|Default|GetParticleSystem) true false)
  (bind _새_트랙_0 (Timeline|타임라인_0 PlayFromStart)
    (:Update
      (Transformation|SetRelativeScale3D (Variables|Default|GetParticleSystem) (Math|Conversions|ToVector(Float) _새_트랙_0)))))

(event EventOnUnequip
  (Components|Activation|SetActive (Variables|Default|GetParticleSystem) false false))

(fn ConstructionScript)