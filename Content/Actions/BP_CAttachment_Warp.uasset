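; Attachment for the Warp action that drives a material effect on the owning character's mesh while it is equipped.
; On equip, it enables the material's panner, sets its speed and plays a timeline that animates the Pow parameter.
; On unequip, the same timeline reverses, and its Finished pin switches the panner off only when the direction is backward, so the effect eases out first.
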(event EventBeginPlay)

(event EventOnEquip
  (bind _ownercharacter (Variables|Default|GetOwnerCharacter))
  (bind _mesh (Variables|/Script/Engine.Character|GetMesh _ownercharacter))
  (Rendering|Material|SetScalarParameterValueonMaterials (Variables|/Script/Engine.Character|GetMesh (Variables|Default|GetOwnerCharacter)) "bUsePanner" 1.0)
  (Rendering|Material|SetScalarParameterValueonMaterials _mesh "Speed" 0.25)
  (bind (_direction _새_트랙_0) (Timeline|타임라인_0 PlayFromStart)
    (:Update
      (Rendering|Material|SetScalarParameterValueonMaterials _mesh "Pow" _새_트랙_0))
    (:Finished
      (if (Utilities|Enum|Equal(Enum) _direction "Backward")
        (Rendering|Material|SetScalarParameterValueonMaterials (Variables|/Script/Engine.Character|GetMesh (Variables|Default|GetOwnerCharacter)) "bUsePanner" 0.0)))))

(event EventOnUnequip
  (bind (_direction _새_트랙_0) (Timeline|타임라인_0 ReverseFromEnd)
    (:Update
      (Rendering|Material|SetScalarParameterValueonMaterials (Variables|/Script/Engine.Character|GetMesh (Variables|Default|GetOwnerCharacter)) "Pow" _새_트랙_0))
    (:Finished
      (if (Utilities|Enum|Equal(Enum) _direction "Backward")
        (Rendering|Material|SetScalarParameterValueonMaterials (Variables|/Script/Engine.Character|GetMesh (Variables|Default|GetOwnerCharacter)) "bUsePanner" 0.0)))))

(fn ConstructionScript)